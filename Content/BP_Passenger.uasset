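; BP_Passenger is a physics-driven passenger that turns toward and moves to points the player clicks.
; It stores click locations broadcast by BP_PlayerController, and each Tick runs RotatePassenger, then MovePassenger.
; Rotation sets angular velocity until IsFacingPoint returns false, then movement applies forward force until the actor nears the target.
; IsFacingPoint, despite gating rotation, shows only an unused yaw-difference comparison.
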(event `self.ReceiveBeginPlay`
  (bind _asbp_player_controller (cast `/Game/BP_PlayerController` (`GameplayStatics.GetPlayerController` 0)))
  (add `/Game/BP_PlayerController.OnMouseClickInValidSpace` _asbp_player_controller (delegate `OnMouseClickInValidSpaceHandler`)))

(event `OnMouseClickInValidSpaceHandler`
  (params (MouseClickLocation :type "Vector Structure"))
  (set `self.MouseClickLocation` MouseClickLocation)
  (set `self.MouseClicked` true))

(event `self.ReceiveTick`
  (params (DeltaSeconds :type "Float (single-precision)"))
  (`|ExecutionSequence`
    (:`then_0`
      (`self.RotatePassenger` DeltaSeconds))
    (:`then_1`
      (`self.MovePassenger` DeltaSeconds))))

(fn `MovePassenger`
  (params (DelataSeconds :type "Float (double-precision)"))
  (locals (DistanceThreshold :type "Float (double-precision)" :default 5.0))
  (if (`self.ReadyToMove`)
    (`PrimitiveComponent.SetPhysicsAngularVelocityInDegrees` (`self.Mesh`) (0.0 0.0 0.0) false "None")
    (if (!= (- (`self.K2_GetActorLocation`) (`self.MouseClickLocation`)) (0.0 0.0 0.0) :`ErrorTolerance` 20.0)
      (`PrimitiveComponent.AddForce` (`self.Mesh`) (* (`SceneComponent.GetForwardVector` (`self.Mesh`)) (`self.Speed`)) "None" false)
      (else
        (set `self.ReadyToMove` false)))))

(fn `RotatePassenger`
  (params (DeltaSeconds :type "Float (double-precision)"))
  (locals (RotateAngle :type "Vector Structure" :default (0.0 0.0 1.0)) (RotateReverseAngle :type "Vector Structure" :default (0.0 0.0 -1.0)))
  (bind (_returnvalue_roll _returnvalue_pitch _returnvalue_yaw) (`KismetMathLibrary.BreakRotator` (`self.K2_GetActorRotation`)))
  (bind (_returnvalue_roll_2 _returnvalue_pitch_2 _returnvalue_yaw_2) (`KismetMathLibrary.BreakRotator` (`KismetMathLibrary.FindLookAtRotation` (`self.K2_GetActorLocation`) (`self.MouseClickLocation`))))
  (bind _returnvalue (- (`KismetMathLibrary.MakeVector` 0.0 0.0 _returnvalue_yaw_2) (`KismetMathLibrary.MakeVector` 0.0 0.0 _returnvalue_yaw)))
  (if (`self.MouseClicked`)
    (if (!= _returnvalue (0.0 0.0 0.0) :`ErrorTolerance` 2.0)
      (`PrimitiveComponent.SetPhysicsAngularVelocityInRadians` (`self.Mesh`) (* (`KismetMathLibrary.Normal` _returnvalue) (/ (`self.Speed`) 100.0)) false "None")
      (set `self.ReadyToMove` false)
      (else
        (`PrimitiveComponent.SetPhysicsAngularVelocityInRadians` (`self.Mesh`) (0.0 0.0 0.0) false "None")
        (set `self.ReadyToMove` true)
        (set `self.MouseClicked` false)))))

(fn `UserConstructionScript`)