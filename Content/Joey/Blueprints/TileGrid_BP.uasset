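; TileGrid_BP is an actor that builds a Rows by Cols grid of Tile_BP actors at its location on BeginPlay.
; An outer loop spawns each row's first tile along world X, and an inner loop spawns the remaining tiles along Y from it.
; Spacing comes from each spawned tile's actor bounds, so tiles sit edge to edge.
; A final pass records each tile's placed location as its StartPosition.
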(event `self.ReceiveBeginPlay`
  (bind (_returnvalue_x _returnvalue_y _returnvalue_z) (`KismetMathLibrary.BreakVector` (`self.K2_GetActorLocation`)))
  (bind _currentxtile (`self.currentXtile`))
  (bind (_returnvalue_x_2 _returnvalue_y_2 _returnvalue_z_2) (`KismetMathLibrary.BreakVector` (`self.K2_GetActorLocation` _currentxtile)))
  ;[1 0 0.4463] Rows
  (for _index (range 1 (+ (`self.rows`) 1))
    (bind _returnvalue (`|SpawnActorFromClass` "/Game/Joey/Blueprints/Tile_BP.Tile_BP_C" (`self.GetTransform`) "Undefined" "OverrideRootScale" null null))
    (bind _output_get (set `self.currentXtile` _returnvalue))
    (`KismetArrayLibrary.Array_Add` (`self.tiles`) _output_get)
    (bind (_center _boxextent) (`GameplayStatics.GetActorArrayBounds` (`|MakeArray` _output_get :!type "Actor Object Reference")))
    (bind _output_get_2 (set `self.currTileLocation` (`KismetMathLibrary.MakeVector` (+ (* (.x _boxextent) (`KismetMathLibrary.Conv_IntToDouble` _index) 2.0) _returnvalue_x) _returnvalue_y _returnvalue_z)))
    (`self.K2_SetActorLocation` (`self.currentXtile`) _output_get_2 false false)
    ;[0 0.3836 1] Columns
    (for _index_2 (range 1 (`self.cols`))
      (bind _returnvalue_2 (`|SpawnActorFromClass` "/Game/Joey/Blueprints/Tile_BP.Tile_BP_C" (`self.GetTransform` _currentxtile) "Undefined" "OverrideRootScale" null null))
      (`KismetArrayLibrary.Array_Add` (`self.tiles`) _returnvalue_2)
      (bind (_center_2 _boxextent_2) (`GameplayStatics.GetActorArrayBounds` (`|MakeArray` _returnvalue_2 :!type "Actor Object Reference")))
      (bind _output_get_3 (set `self.currTileLocation` (`KismetMathLibrary.MakeVector` _returnvalue_x_2 (+ (* (.y _boxextent_2) (`KismetMathLibrary.Conv_IntToDouble` _index_2) 2.0) _returnvalue_y_2) _returnvalue_z_2)))
      (`self.K2_SetActorLocation` _returnvalue_2 _output_get_3 false false)))
  (for _array_element (`self.tiles`)
    (bind _astile_bp (cast `/Game/Joey/Blueprints/Tile_BP` _array_element))
    (set `/Game/Joey/Blueprints/Tile_BP.StartPosition` (`self.K2_GetActorLocation` _astile_bp) _astile_bp)))

(fn `UserConstructionScript`
  (set `self.rows` (`self.rows`))
  (set `self.cols` (`self.cols`)))